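; Moving platform actor that glides once to an offset position when the player steps into its trigger box.
; BeginPlay stores the end location from the starting position plus Offset and disables tick.
; A player pawn overlap re-enables tick, which eases the actor toward the target with VInterpTo and switches itself off again when within a small distance.
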(event OnComponentBeginOverlap(Box)
  (params (OverlappedComponent :type Primitive%20Component%20Object%20Reference) (OtherActor :type Actor%20Object%20Reference) (OtherComp :type Primitive%20Component%20Object%20Reference) (OtherBodyIndex :type Integer) (bFromSweep :type Boolean) (SweepResult :type Hit%20Result%20Structure%20%28by%20ref%29))
  (if (== OtherActor (Game|Player|GetPlayerPawn 0))
    (Actor|Tick|SetActorTickEnabled true)))

(event EventTick
  (params (DeltaSeconds :type Float%20%28single-precision%29))
  (Transformation|SetActorLocation (Math|Interpolation|VInterpTo (Transformation|GetActorLocation) (Variables|Default|GetEndLocation) DeltaSeconds (Variables|Default|GetInterp%20Speed)) false false)
  (if (< (Math|Vector|VectorLength (- (Variables|Default|GetEndLocation) (Transformation|GetActorLocation))) 5.0)
    (Actor|Tick|SetActorTickEnabled false)))

(event EventBeginPlay
  ;[1 1 1] Calculate end location.
  (Variables|Default|SetEndLocation (+ (Transformation|GetActorLocation) (Variables|Default|GetOffset)))
  (Actor|Tick|SetActorTickEnabled false))

(fn ConstructionScript)